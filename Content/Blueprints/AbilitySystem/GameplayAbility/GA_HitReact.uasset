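; Gameplay ability that plays the avatar's hit-react montage when activated.
; After committing, it gets the montage through the UR_CombatInterface and applies GE_HitReact to itself as playback starts.
; When the montage completes, is interrupted or is cancelled, it removes effects tagged Effects.HitReact and ends.
; A failed commit, failed cast or invalid montage leaves the graph without calling EndAbility.
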(event `self.K2_ActivateAbility`
  (bind _returnvalue (`self.K2_CommitAbility`))
  (if _returnvalue
    (bind _asaur_combat_interface (cast `AUR_CombatInterface` (`self.GetAvatarActorFromActorInfo`)))
    (bind _returnvalue_2 (`AUR_CombatInterface.GetHitReactMontage` _asaur_combat_interface))
    (`/Engine/EditorBlueprintResources/StandardMacros.IsValid` _returnvalue_2
      (:`Is Valid`
        (`AbilityTask_PlayMontageAndWait.CreatePlayMontageAndWaitProxy` "None" _returnvalue_2
          (:`then`
            (`AbilitySystemComponent.BP_ApplyGameplayEffectToSelf` :`self` (`self.GetAbilitySystemComponentFromActorInfo`) :`GameplayEffectClass` "/Game/Blueprints/AbilitySystem/GameplayEffects/GE_HitReact.GE_HitReact_C"))
          (:`OnCompleted`
            (`AbilitySystemComponent.RemoveActiveEffectsWithTags` (`self.GetAbilitySystemComponentFromActorInfo`) (struct :`GameplayTags` (struct :`(TagName` "Effects.HitReact"))) :!label _label)
            (`self.K2_EndAbility`))
          (:`OnInterrupted`
            (goto _label))
          (:`OnCancelled`
            (goto _label)))))))